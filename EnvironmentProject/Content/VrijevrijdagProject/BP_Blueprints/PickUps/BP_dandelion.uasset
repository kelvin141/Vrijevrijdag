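; BP_dandelion is a physics-driven dandelion pickup that can be carried and dropped.
; Pickup turns off mesh physics, attaches the actor to the given component and stores the attach result as PickedUp; Drop restores physics, detaches and clears the flag.
; It enables player input on BeginPlay so the LetDandelionsfly action calls DandelionsLose while held, though that event is empty in this graph.
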(event Custom|dandelionsLose)

(event EventBeginPlay
  (Input|EnableInput (Game|GetPlayerController 0)))

(event Collision|EventActorBeginOverlap
  (params (OtherActor :type Actor%20Object%20Reference)))

(event EventTick
  (params (DeltaSeconds :type Float%20%28single-precision%29)))

(event EventPickup
  (params (AttachTo :type Scene%20Component%20Object%20Reference))
  (Physics|SetSimulatePhysics (Variables|Debug|GetStaticMeshComponent) false)
  (bind _returnvalue (Transformation|AttachComponentToComponent (VehicleSound|GetRootComponent) AttachTo "None" "KeepWorld" "KeepWorld" "KeepWorld" false))
  (Variables|Default|SetPickedUp _returnvalue))

(event EventDrop
  (Physics|SetSimulatePhysics (Variables|Debug|GetStaticMeshComponent) true)
  (Transformation|DetachFromActor "KeepWorld" "KeepWorld" "KeepWorld")
  (Variables|Default|SetPickedUp false))

(event Input|ActionEvents|InputActionLetDandelionsfly
  (params (Key :type Key%20Structure :default "None"))
  (:Pressed
    (if (Variables|Default|GetPickedUp)
      (CallFunction|DandelionsLose))))

(fn ConstructionScript)